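; BP_LevelFalloff is a trigger volume that handles the player marble, BP_Marbo, falling off the level.
; On box overlap it waits briefly, then disables physics simulation on the marble mesh.
; If the marble's GetMarbleDeath returns true, it teleports the marble to a stored Location and re-enables physics; otherwise it reloads the current level by name.
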(event OnComponentBeginOverlap(Box)
  (params (OverlappedComponent :type Primitive%20Component%20Object%20Reference) (OtherActor :type Actor%20Object%20Reference) (OtherComp :type Primitive%20Component%20Object%20Reference) (OtherBodyIndex :type Integer) (bFromSweep :type Boolean) (SweepResult :type Hit%20Result%20Structure%20%28by%20ref%29))
  (bind _asbp_marbo (Utilities|Casting|CastToBP_Marbo OtherActor))
  (Utilities|FlowControl|Delay 0.2)
  (Physics|SetSimulatePhysics (Variables|/Script/RMarboR.Marble|GetMarbleMesh _asbp_marbo) false)
  (bind _returnvalue (Class|Marble|GetMarbleDeath _asbp_marbo))
  (if _returnvalue
    (Transformation|SetActorLocation _asbp_marbo (Variables|Default|GetLocation) false true)
    (Physics|SetSimulatePhysics (Variables|/Script/RMarboR.Marble|GetMarbleMesh _asbp_marbo) true)
    (else
      (bind _returnvalue_2 (Game|GetCurrentLevelName true))
      (Game|OpenLevel(byName) (Utilities|String|StringToName _returnvalue_2)))))

(event EventBeginPlay)

(event Collision|EventActorBeginOverlap
  (params (OtherActor :type Actor%20Object%20Reference)))

(event EventTick
  (params (DeltaSeconds :type Float%20%28single-precision%29)))

(fn ConstructionScript)