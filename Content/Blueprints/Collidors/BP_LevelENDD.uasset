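; BP_LevelENDD is a level exit trigger that loads the level named by LevelName once no gems remain.
; When a BP_Marbo enters its Box, it counts the BP_Gem actors still in the world.
; If any remain, it shows a WBP_GemMiss widget for three seconds instead of changing level.
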(event OnComponentBeginOverlap(Box)
  (params (OverlappedComponent :type Primitive%20Component%20Object%20Reference) (OtherActor :type Actor%20Object%20Reference) (OtherComp :type Primitive%20Component%20Object%20Reference) (OtherBodyIndex :type Integer) (bFromSweep :type Boolean) (SweepResult :type Hit%20Result%20Structure%20%28by%20ref%29))
  (Utilities|Casting|CastToBP_Marbo OtherActor)
  (bind _outactors (Actor|GetAllActorsOfClass "/Game/Blueprints/Collectiblles/BP_Gem.BP_Gem_C"))
  (if (> (Utilities|Array|Length _outactors) 0)
    (bind _returnvalue (UserInterface|CreateWidget "/Game/Blueprints/UI/WBP_GemMiss.WBP_GemMiss_C"))
    (UserInterface|Viewport|AddtoViewport _returnvalue 0)
    (Utilities|FlowControl|Delay 3.0)
    (Widget|RemovefromParent _returnvalue)
    (else
      (Game|OpenLevel(byName) (Variables|Default|GetLevel%20Name)))))

(event EventBeginPlay)

(event Collision|EventActorBeginOverlap
  (params (OtherActor :type Actor%20Object%20Reference)))

(event EventTick
  (params (DeltaSeconds :type Float%20%28single-precision%29)))

(fn ConstructionScript)